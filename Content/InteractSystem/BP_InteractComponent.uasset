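; Player interaction component that finds the interactable in view and highlights it with a custom depth stencil outline.
; Each tick it line-traces from the player camera on Visibility and tracks hit actors implementing the Interactable interface.
; Static meshes of the current target get one of two stencil values, depending on whether CanInteractMessage passes.
; ForwardInteractInput calls OnInteractMessage on that target only while the check is true.
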(event Custom|Forward%20Interact%20Input
  (if (and (Utilities|IsValid (Variables|Default|GetCurrent%20Interactable)) (Variables|Default|GetLast%20Computed%20Condition))
    (Class|Interactable|OnInteract(Message) (Variables|Default|GetCurrent%20Interactable))))

(event EventBeginPlay
  (bind _asbp_player (Utilities|Casting|CastToBP_Player (Components|GetOwner)))
  (bind _output_get (Variables|Default|SetOwning%20Player _asbp_player))
  (Variables|Default|SetOwning%20Camera (Variables|/Game/BP_Player.BP_Player_C|GetCamera _output_get))
  (Components|Tick|SetComponentTickEnabled true))

(event EventTick
  (params (DeltaSeconds :type Float%20%28single-precision%29))
  (bind _updated (CallFunction|UpdateInteraction))
  (if _updated
    (CallFunction|EnableOutline (Variables|Default|GetCurrent%20Interactable) 1)
    (Variables|Default|SetLast%20Computed%20Condition false))
  (bind _bcaninteract_ (Class|Interactable|CanInteract(Message) (Variables|Default|GetCurrent%20Interactable)))
  (if (!= _bcaninteract_ (Variables|Default|GetLast%20Computed%20Condition))
    (Variables|Default|SetLast%20Computed%20Condition _bcaninteract_)
    (CallFunction|EnableOutline (Variables|Default|GetCurrent%20Interactable) (Math|Integer|SelectInt 2 1 (Variables|Default|GetLast%20Computed%20Condition)))))

(fn UpdateInteraction
  (bind _owning_camera (Variables|Default|GetOwning%20Camera))
  (bind _returnvalue (Transformation|GetWorldLocation _owning_camera))
  (bind (_outhit _returnvalue_2) (Collision|LineTraceByChannel _returnvalue (+ _returnvalue (* (Math|Vector|GetForwardVector _owning_camera) (Variables|Default|GetInteract%20Max%20Distance))) "TraceTypeQuery1" false (Utilities|Array|MakeArray (Variables|Default|GetOwning%20Player)) "None"))
  (if (and _returnvalue_2 (Utilities|DoesObjectImplementInterface (.HitActor (Collision|BreakHitResult _outhit)) "/Game/InteractSystem/Interactable.Interactable_C"))
    (bind _output_get (LocalVariables|SetHit%20Actor (.HitActor (Collision|BreakHitResult _outhit))))
    (if (!= _output_get (Variables|Default|GetCurrent%20Interactable))
      (Utilities|FlowControl|Sequence
        (:then_0
          (Utilities|IsValid (Variables|Default|GetCurrent%20Interactable)
            (:Is%20Valid
              (CallFunction|DisableOutline (Variables|Default|GetCurrent%20Interactable)))))
        (:then_1
          (Variables|Default|SetCurrent%20Interactable (LocalVariables|GetHit%20Actor))
          (return true)))
      (else
        (return false)))
    (else
      (Utilities|IsValid (Variables|Default|GetCurrent%20Interactable)
        (:Is%20Valid
          (CallFunction|DisableOutline (Variables|Default|GetCurrent%20Interactable))
          (Variables|Default|SetCurrent%20Interactable 0)
          (return true))
        (:Is%20Not%20Valid
          (return false))))))

(fn EnableOutline
  (params (Interactable :type Actor%20Object%20Reference) (Value :type Integer))
  (Utilities|IsValid Interactable
    (:Is%20Valid
      (for _array_element (Actor|GetComponentsByClass Interactable "/Script/Engine.StaticMeshComponent")
        (Rendering|SetCustomDepthStencilValue _array_element Value)
        (Rendering|SetRenderCustomDepth _array_element true)))))

(fn DisableOutline
  (params (Interactable :type Actor%20Object%20Reference))
  (for _array_element (Actor|GetComponentsByClass Interactable "/Script/Engine.StaticMeshComponent")
    (Rendering|SetCustomDepthStencilValue _array_element 0)
    (Rendering|SetRenderCustomDepth _array_element false)))