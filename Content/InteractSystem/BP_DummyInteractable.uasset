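; BP_DummyInteractable is a placeholder interactable actor that launches vertically when interacted with.
; After a short delay from BeginPlay it enables interaction and activates a cosmic projectile particle effect, having cached its start location.
; OnInteract clears the CanInteract flag and plays the Launch timeline, which offsets the actor's Z from that start location without sweeping.
; The flag is never re-enabled, so interaction is one-shot.
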(event EventBeginPlay
  (Variables|Default|SetStart%20Location (Transformation|GetActorLocation))
  (Utilities|FlowControl|Delay 5.0)
  (Variables|Default|SetCan%20Interact%20? true)
  (Components|Activation|Activate (Variables|Default|GetP_Cosmic_Projectile_03) true))

(event EventOnInteract
  (Variables|Default|SetCan%20Interact%20? false)
  (bind _delta_z (Timeline|Launch Play)
    (:Update
      (Transformation|SetActorLocation (+ (Variables|Default|GetStart%20Location) (Math|Vector|MakeVector 0.0 0.0 _delta_z)) false false))))

(fn ConstructionScript)

(fn CanInteract
  (return (Variables|Default|GetCan%20Interact%20?)))